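; BP_Base is a faction base actor that triggers a resource transaction when a send character of the same faction reaches it.
; Its Box overlap accepts only the capsule component of a BP_SendCharacter_Base whose faction matches the base's.
; It passes that unit's UnitTax to HandleTransaction on the first player controller's ResourceComponent.
; The transaction always targets that player, as per-faction switching awaits AI implementation.
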(event `self.Box.OnComponentBeginOverlap`
  (params (OverlappedComponent :type "PrimitiveComponent Object Reference") (OtherActor :type "Actor Object Reference") (OtherComp :type "PrimitiveComponent Object Reference") (OtherBodyIndex :type Integer) (bFromSweep :type Boolean) (SweepResult :type "HitResult Structure (by ref)"))
  (bind _asbp_send_character_base (cast `/Game/Characters/Sends/BP_SendCharacter_Base` OtherActor))
  (if (and (`|EnumEquality` (`SendCharacter.FactionType` _asbp_send_character_base) (`self.Faction`)) (== OtherComp (`Character.CapsuleComponent` _asbp_send_character_base)))
    (`ResourceComponent.HandleTransaction` (`GrowthPlayerController.ResourceComponent` (cast `/Game/BP_MainPlayerController` (`GameplayStatics.GetPlayerController` 0) :!pure true)) (`SendCharacter.UnitTax` _asbp_send_character_base))))

(fn `UserConstructionScript`)
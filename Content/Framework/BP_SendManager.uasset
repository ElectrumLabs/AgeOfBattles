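; Send manager that queues units for training and spawns them for its Friendly or Enemy faction.
; A single timer runs for the head item's training time, then spawns its character at that faction's fixed location with the queued stats and upgrade manager reference.
; Removing the head, by spawning or by index, restarts the timer for the next item.
; Queue changes call an update notification.
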(event `RemoveFromQueueAtIndex`
  (params (IndexToRemove :type Integer))
  (`KismetArrayLibrary.Array_Remove` (`self.SendQueue`) IndexToRemove)
  (if (== IndexToRemove 0)
    (`KismetSystemLibrary.K2_ClearAndInvalidateTimerHandle` (`self.SendTimerHandle`))
    (`self.HandleSendout`))
  (`self.OnUpdateQueue`))

(event `AddToQueue`
  (params (NewItem :type "SendInformation Structure (by ref)"))
  (`KismetArrayLibrary.Array_Add` (`self.SendQueue`) NewItem)
  (`self.HandleSendout`)
  (`self.OnUpdateQueue`))

(event `HandleSendout`
  (bind (_output_unitimage _output_sendname _output_unittype _output_unittier _output_sendcharacter _output_trainingtime) (break `SendInformation` (`|GetArrayItem` (`self.SendQueue`))))
  (if (> (`KismetArrayLibrary.Array_Length` (`self.SendQueue`)) 0)
    (if (not (`KismetSystemLibrary.K2_IsTimerActiveHandle` (`self.SendTimerHandle`)))
      (bind _returnvalue (`KismetSystemLibrary.K2_SetTimerDelegate` (delegate `SpawnSend`) _output_trainingtime))
      (set `self.SendTimerHandle` _returnvalue))))

(event `SpawnSend`
  (bind _factiontype (`self.FactionType`))
  (bind (_output_unitimage _output_sendname _output_unittype _output_unittier _output_sendcharacter _output_trainingtime _output_supplycost _output_resourcecost _output_maximumhealth _output_attackrange _output_attackdamage _output_attackpenetration _output_armor _output_attackspeed _output_unittax _output_goldbounty) (break `SendInformation` (`|GetArrayItem` (`self.SendQueue`))))
  (`|SpawnActorFromClass` _output_sendcharacter (`KismetMathLibrary.MakeTransform` (select `EFactionType` _factiontype :`Friendly` (-4700.0 0.0 150.0) :`Enemy` (4700.0 0.0 150.0) :!type "Vector Structure")) "AdjustIfPossibleButAlwaysSpawn" "OverrideRootScale" null (`self.UpgradeManagerREF`) _output_unittype _output_unittier _output_maximumhealth _output_attackrange _output_attackdamage _output_attackpenetration _output_armor _output_attackspeed _factiontype _output_unittax _output_goldbounty _output_supplycost null)
  (`self.RemoveFromQueueAtIndex` 0)
  (`KismetSystemLibrary.K2_ClearAndInvalidateTimerHandle` (`self.SendTimerHandle`))
  (`self.HandleSendout`)
  (`self.OnUpdateQueue`))
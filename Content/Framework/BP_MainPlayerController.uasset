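; Player controller for a base-versus-base game where the player buys units and upgrades against an enemy controller.
; On play it configures the send manager as friendly, links the upgrades component and shows the HUD, while Escape toggles the pause menu.
; Unit purchases and cancellations adjust resources and supply and edit the send queue, with affordability and upgrade checks.
; An end-game check pauses and shows Defeat or Victory when either base health reaches zero.
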(event `self.ReceiveBeginPlay`
  (set `SendManager.FactionType` "Friendly" (`self.BP_SendManager`))
  (set `/Game/Framework/BP_SendManager.UpgradeManagerREF` (`self.UpgradesComponent`) (`self.BP_SendManager`))
  (bind _returnvalue (`|CreateWidget` "/Game/Widgets/WBP_PlayerHUD.WBP_PlayerHUD_C"))
  (`UserWidget.AddToViewport` _returnvalue 0))

(event `Key|Escape` :paused true
  (params (Key :type "Key Structure"))
  (:`Pressed`
    (if (`self.bGamePaused`)
      (`self.UnpauseGame`)
      (else
        (`self.PauseGame`)))))

(event `PauseGame`
  (`GameplayStatics.SetGamePaused` true)
  (set `self.bGamePaused` true)
  (bind _returnvalue (`|CreateWidget` "/Game/Widgets/MainMenuAndPause/WBP_GamePaused.WBP_GamePaused_C"))
  (set `self.GamePausedWBP` _returnvalue)
  (`UserWidget.AddToViewport` (`self.GamePausedWBP`) 0))

(event `UnpauseGame`
  (bind _gamepausedwbp (`self.GamePausedWBP`))
  (`GameplayStatics.SetGamePaused` false)
  (set `self.bGamePaused` false)
  (`/Engine/EditorBlueprintResources/StandardMacros.IsValid` _gamepausedwbp
    (:`Is Valid`
      (`Widget.RemoveFromParent` _gamepausedwbp))))

(event `CheckIfEndGame`
  (if (<= (`ResourceComponent.ReturnCurrentBaseHealth` (`self.ResourceComponent`)) 0.0)
    (`GameplayStatics.SetGamePaused` true)
    (bind _returnvalue (`|CreateWidget` "/Game/Widgets/MainMenuAndPause/WBP_Defeat.WBP_Defeat_C"))
    (`UserWidget.AddToViewport` _returnvalue 0)
    (else
      (bind _returnvalue_2 (`GameplayStatics.GetActorOfClass` "/Game/EnemyAI/BP_EnemyController.BP_EnemyController_C"))
      (if (<= (`ResourceComponent.ReturnCurrentBaseHealth` (`EnemyController.ResourceComponent` _returnvalue_2)) 0.0)
        (`GameplayStatics.SetGamePaused` true)
        (bind _returnvalue_3 (`|CreateWidget` "/Game/Widgets/MainMenuAndPause/WBP_Victory.WBP_Victory_C"))
        (`UserWidget.AddToViewport` _returnvalue_3 0)))))

(fn `FBuyUnit`
  (params (IncomingSendInfo :type "SendInformation Structure (by ref)"))
  (locals (SendInfo :type "SendInformation Structure"))
  (bind (_sendinfo_unitimage _sendinfo_sendname _sendinfo_unittype _sendinfo_unittier _sendinfo_sendcharacter _sendinfo_trainingtime _sendinfo_supplycost _sendinfo_resourcecost) (break `SendInformation` (`local.SendInfo`)))
  (set `local.SendInfo` IncomingSendInfo)
  (`ResourceComponent.HandleBuy` (`self.ResourceComponent`) _sendinfo_resourcecost)
  (`ResourceComponent.DeltaCurrentSupply` (`self.ResourceComponent`) _sendinfo_supplycost)
  (`/Game/Framework/BP_SendManager.AddToQueue` (`self.BP_SendManager`) (`local.SendInfo`)))

(fn `FCanBuyUnit`
  (params (IncomingSend :type "SendInformation Structure"))
  (returns (ReturnValue :type Boolean))
  (return (and (`ResourceComponent.bCheckIfCanAfford` (`self.ResourceComponent`) IncomingSend_ResourceCost) (`ResourceComponent.bCheckIfSupplyFits` (`self.ResourceComponent`) IncomingSend_SupplyCost) (`SendManager.CanAddToQueue` (`self.BP_SendManager`)))))

(fn `FCancelUnit`
  (params (IncomingSendInfo :type "SendInformation Structure (by ref)") (IndexToRemove :type Integer))
  (locals (SendInfo :type "SendInformation Structure"))
  (bind (_sendinfo_unitimage _sendinfo_sendname _sendinfo_unittype _sendinfo_unittier _sendinfo_sendcharacter _sendinfo_trainingtime _sendinfo_supplycost _sendinfo_resourcecost) (break `SendInformation` (`local.SendInfo`)))
  (set `local.SendInfo` IncomingSendInfo)
  (`ResourceComponent.HandleSell` (`self.ResourceComponent`) _sendinfo_resourcecost)
  (`ResourceComponent.DeltaCurrentSupply` (`self.ResourceComponent`) (* _sendinfo_supplycost -1))
  (`/Game/Framework/BP_SendManager.RemoveFromQueueAtIndex` (`self.BP_SendManager`) IndexToRemove))

(fn `FCanUpgrade`
  (params (Selection :type "UpgradeType Enum" :default "AttackRange"))
  (returns (ReturnValue :type Boolean))
  (locals (Return :type Boolean :default false))
  (switch `UpgradeType` Selection
    (:`AttackRange`
      (set `local.Return` (`self.BCanUpgradeAttackRange`)))
    (:`AttackDamage`
      (set `local.Return` (`self.BCanUpgradeAttackDamage`)))
    (:`AttackPenetration`
      (set `local.Return` (`self.BCanUpgradeAttackPenetration`)))
    (:`Armor`
      (set `local.Return` (`self.BCanUpgradeArmor`)))
    (:`AttackSpeed`
      (set `local.Return` (`self.BCanUpgradeAttackSpeed`))))
  (return (`local.Return`)))

(fn `UserConstructionScript`)
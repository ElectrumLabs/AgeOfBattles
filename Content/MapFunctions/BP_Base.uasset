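; Faction base on the map that collects the UnitTax of same-faction send characters entering its trigger box.
; The box overlap accepts only the unit's capsule, then passes the tax to HandleSell on the ResourceComponent of the player controller (Friendly) or BP_EnemyController (Enemy).
; For friendly units, FHandleResourceNumbers also spawns one BP_ResourceGain per resource type at a random offset above the unit to show the amount.
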(event `self.Box.OnComponentBeginOverlap`
  (params (OverlappedComponent :type "PrimitiveComponent Object Reference") (OtherActor :type "Actor Object Reference") (OtherComp :type "PrimitiveComponent Object Reference") (OtherBodyIndex :type Integer) (bFromSweep :type Boolean) (SweepResult :type "HitResult Structure (by ref)"))
  (bind _asbp_send_character_base (cast `/Game/Characters/Sends/BP_SendCharacter_Base` OtherActor))
  (if (and (`|EnumEquality` (`SendCharacter.FactionType` _asbp_send_character_base) (`self.Faction`)) (== OtherComp (`Character.CapsuleComponent` _asbp_send_character_base)))
    (switch `EFactionType` (`self.Faction`)
      (:`Friendly`
        (bind _unittax (`SendCharacter.UnitTax` _asbp_send_character_base))
        (`ResourceComponent.HandleSell` (`GrowthPlayerController.ResourceComponent` (cast `/Game/Framework/BP_MainPlayerController` (`GameplayStatics.GetPlayerController` 0) :!pure true)) _unittax)
        (`self.FHandleResourceNumbers` _unittax _asbp_send_character_base))
      (:`Enemy`
        (bind _returnvalue (`GameplayStatics.GetActorOfClass` "/Game/EnemyAI/BP_EnemyController.BP_EnemyController_C"))
        (`ResourceComponent.HandleSell` (`EnemyController.ResourceComponent` _returnvalue) _unittax)))))

(fn `FHandleResourceNumbers`
  (params (ResourceMap :type "Map of ResourceType Enum to Float (single-precision)") (Target :type "Actor Object Reference"))
  (bind (_returnvalue_x _returnvalue_y _returnvalue_z) (`KismetMathLibrary.BreakVector` (`self.K2_GetActorLocation` Target)))
  (bind _keys (`BlueprintMapLibrary.Map_Keys` ResourceMap))
  (bind _values (`BlueprintMapLibrary.Map_Values` ResourceMap))
  (for (_array_element _array_index) _keys
    (`|SpawnActorFromClass` "/Game/Widgets/UnitTooltip/BP_ResourceGain.BP_ResourceGain_C" (`KismetMathLibrary.MakeTransform` (`KismetMathLibrary.MakeVector` (+ _returnvalue_x (`KismetMathLibrary.RandomFloatInRange` -40.0 40.0)) (+ _returnvalue_y (`KismetMathLibrary.RandomFloatInRange` -40.0 40.0)) (+ _returnvalue_z (`KismetMathLibrary.RandomFloatInRange` 100.0 300.0)))) "Undefined" "OverrideRootScale" null _array_element (`KismetMathLibrary.FTrunc` (`|GetArrayItem` _values _array_index)) null)))

(fn `UserConstructionScript`)
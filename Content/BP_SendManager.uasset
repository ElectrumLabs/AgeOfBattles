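; BP_SendManager manages a queue of character sends, releasing them one at a time after each item's training time.
; Adding an item starts a one-shot timer for the front entry if none is running.
; When it fires, it spawns that entry's character class at a hard-coded location, removes it from the queue and starts timing the next.
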(event `AddToQueue`
  (params (NewItem :type "SendInformation Structure (by ref)"))
  (`KismetArrayLibrary.Array_Add` (`self.SendQueue`) NewItem)
  (`self.HandleSendout`))

(event `HandleSendout`
  (bind (_output_sendcharacter _output_trainingtime) (break `SendInformation` (`|GetArrayItem` (`self.SendQueue`))))
  (if (> (`KismetArrayLibrary.Array_Length` (`self.SendQueue`)) 0)
    (if (not (`KismetSystemLibrary.K2_IsTimerActiveHandle` (`self.SendTimerHandle`)))
      (bind _returnvalue (`KismetSystemLibrary.K2_SetTimerDelegate` (delegate `SpawnSend`) _output_trainingtime))
      (set `self.SendTimerHandle` _returnvalue))))

(event `SpawnSend`
  (bind _output_sendcharacter (break `SendInformation` (`|GetArrayItem` (`self.SendQueue`))))
  (`KismetSystemLibrary.K2_ClearAndInvalidateTimerHandle` (`self.SendTimerHandle`))
  ;[1 1 1] hc atm
  (`|SpawnActorFromClass` _output_sendcharacter (`KismetMathLibrary.MakeTransform` (-4700.0 0.0 100.0)) "AdjustIfPossibleButAlwaysSpawn" "OverrideRootScale" null "Friendly" null)
  (`self.RemoveFromQueueAtIndex` 0)
  (`self.HandleSendout`))

(event `RemoveFromQueueAtIndex`
  (params (IndexToRemove :type Integer))
  (`KismetArrayLibrary.Array_Remove` (`self.SendQueue`) IndexToRemove))
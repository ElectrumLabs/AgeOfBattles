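; Base class for faction-based send units that automatically attack opposing sends and carry gold bounty and supply cost.
; Two overlap spheres track nearby and in-range enemies; a looping timer plays a melee or ranged montage, or sets Moving and re-queries targets.
; DamageGate hits the first in-range enemy using level-indexed stats.
; Damage spawns floating numbers; death frees the owner's supply, pays the opposing controller and refreshes the killer's targets.
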(event `self.ReceiveBeginPlay`
  (`parent.ReceiveBeginPlay`)
  (`self.HandleAttackTimer`))

(event `self.AttackIndicator.OnComponentBeginOverlap`
  (params (OverlappedComponent :type "PrimitiveComponent Object Reference") (OtherActor :type "Actor Object Reference") (OtherComp :type "PrimitiveComponent Object Reference") (OtherBodyIndex :type Integer) (bFromSweep :type Boolean) (SweepResult :type "HitResult Structure (by ref)"))
  (if (== (`KismetSystemLibrary.GetObjectName` OtherComp) (`KismetSystemLibrary.GetObjectName` (`self.Box`)))
    (bind _asbp_send_character_base (cast `/Game/Characters/Sends/BP_SendCharacter_Base` OtherActor))
    (if (`|EnumInequality` (`SendCharacter.FactionType` _asbp_send_character_base) (`self.FactionType`))
      (`KismetArrayLibrary.Array_AddUnique` (`self.EnemiesInRange`) _asbp_send_character_base))))

(event `self.FindIndicator.OnComponentBeginOverlap`
  (params (OverlappedComponent :type "PrimitiveComponent Object Reference") (OtherActor :type "Actor Object Reference") (OtherComp :type "PrimitiveComponent Object Reference") (OtherBodyIndex :type Integer) (bFromSweep :type Boolean) (SweepResult :type "HitResult Structure (by ref)"))
  (if (== (`KismetSystemLibrary.GetObjectName` OtherComp) (`KismetSystemLibrary.GetObjectName` (`self.Box`)))
    (bind _asbp_send_character_base (cast `/Game/Characters/Sends/BP_SendCharacter_Base` OtherActor))
    (if (`|EnumInequality` (`SendCharacter.FactionType` _asbp_send_character_base) (`self.FactionType`))
      (`KismetArrayLibrary.Array_AddUnique` (`self.EnemyArray`) _asbp_send_character_base))))

(event `HandleAttackTimer`
  (`KismetSystemLibrary.K2_SetTimerDelegate` (delegate `HandleAttack`) 0.2 true))

(event `HandleAttack`
  (if (not (`self.bIsAttacking`))
    (`self.Attack`)))

(event `Attack`
  (`/Engine/EditorBlueprintResources/StandardMacros.IsValid` (`|GetArrayItem` (`self.EnemiesInRange`))
    (:`Is Valid`
      (set `self.SendState` "Attacking")
      (set `self.bIsAttacking` true)
      (`|PlayMontage` (`self.Hands`) (select `EWeaponType` (`self.WeaponType`) :`Melee` "/Game/hs03_ModularHero/Animations/AM_MeleeAttack.AM_MeleeAttack" :`Ranged` "/Game/hs03_ModularHero/Animations/AM_RangedAttack.AM_RangedAttack" :!type "AnimMontage Object Reference") (`|GetArrayItem` (`self.AttackSpeed`) (`self.AttackSpeedLevel`))
        (:`OnCompleted`
          (set `self.bIsAttacking` false))))
    (:`Is Not Valid`
      (set `self.SendState` "Moving")
      (`self.FQueryTargets`))))

(event `DamageGate`
  (bind _output (`|GetArrayItem` (`self.EnemiesInRange`)))
  (`/Engine/EditorBlueprintResources/StandardMacros.IsValid` _output
    (:`Is Valid`
      (bind _asbp_send_character_base (cast `/Game/Characters/Sends/BP_SendCharacter_Base` _output))
      (`self.HandleDamage` _asbp_send_character_base (`|GetArrayItem` (`self.AttackDamage`) (`self.AttackDamageLevel`)) (`|GetArrayItem` (`self.AttackPenetration`) (`self.AttackPenetrationLevel`)) self))))

(event `self.K2_PostDamageEvent`
  (params (FinalDamage :type "Float (single-precision)") (InstigatingSend :type "SendCharacter Object Reference"))
  (`|SpawnActorFromClass` "/Game/Widgets/BP_DamageNumbersActor.BP_DamageNumbersActor_C" (`KismetMathLibrary.MakeTransform` (`self.K2_GetActorLocation`)) "Undefined" "OverrideRootScale" null FinalDamage null)
  (if (not (> (`self.CurrentHealth`) 0.0))
    (`self.DecreaseSupply`)
    (bind _asbp_send_character_base (cast `/Game/Characters/Sends/BP_SendCharacter_Base` InstigatingSend)
      (:`then`
        (`self.FQueryTargets` _asbp_send_character_base)
        (`self.AddGoldToOwner` _asbp_send_character_base (`self.GoldBounty`) (`self.FactionType`)))
      (:`CastFailed`
        _))
    (`self.K2_DestroyActor`)))

(event `AddGoldToOwner`
  (params (DeltaNum :type "Float (single-precision)") (Selection :type "EFactionType Enum" :default "Friendly"))
  (switch `EFactionType` Selection
    (:`Friendly`
      (bind _returnvalue (`GameplayStatics.GetActorOfClass` "/Game/EnemyAI/BP_EnemyController.BP_EnemyController_C"))
      (`ResourceComponent.DeltaGold` (`EnemyController.ResourceComponent` _returnvalue) DeltaNum))
    (:`Enemy`
      (bind _asbp_main_player_controller (cast `/Game/Framework/BP_MainPlayerController` (`GameplayStatics.GetPlayerController` 0)))
      (`ResourceComponent.DeltaGold` (`GrowthPlayerController.ResourceComponent` _asbp_main_player_controller) DeltaNum))))

(event `DecreaseSupply`
  (switch `EFactionType` (`self.FactionType`)
    (:`Friendly`
      (bind _asbp_main_player_controller (cast `/Game/Framework/BP_MainPlayerController` (`GameplayStatics.GetPlayerController` 0)))
      (`ResourceComponent.DeltaCurrentSupply` (`GrowthPlayerController.ResourceComponent` _asbp_main_player_controller) (* (`self.SupplyCost`) -1)))
    (:`Enemy`
      (bind _returnvalue (`GameplayStatics.GetActorOfClass` "/Game/EnemyAI/BP_EnemyController.BP_EnemyController_C"))
      (`ResourceComponent.DeltaCurrentSupply` (`EnemyController.ResourceComponent` _returnvalue) (* (`self.SupplyCost`) -1)))))

(fn `FPlayAttackAnimation`
  (for _ (`SceneComponent.GetChildrenComponents` (`self.Mesh`) false)
    _))

(fn `FQueryTargets`
  (`KismetArrayLibrary.Array_Clear` (`self.EnemyArray`))
  (for _array_element (`PrimitiveComponent.GetOverlappingComponents` (`self.FindIndicator`))
    (if (== (`KismetSystemLibrary.GetObjectName` _array_element) (`KismetSystemLibrary.GetObjectName` (`self.Box`)))
      (bind _asbp_send_character_base (cast `/Game/Characters/Sends/BP_SendCharacter_Base` (`ActorComponent.GetOwner` _array_element)))
      (if (`|EnumInequality` (`SendCharacter.FactionType` _asbp_send_character_base) (`self.FactionType`))
        (`KismetArrayLibrary.Array_AddUnique` (`self.EnemyArray`) _asbp_send_character_base))))
  (`KismetArrayLibrary.Array_Clear` (`self.EnemiesInRange`))
  (for _array_element_2 (`PrimitiveComponent.GetOverlappingComponents` (`self.AttackIndicator`))
    (if (== (`KismetSystemLibrary.GetObjectName` _array_element_2) (`KismetSystemLibrary.GetObjectName` (`self.Box`)))
      (bind _asbp_send_character_base_2 (cast `/Game/Characters/Sends/BP_SendCharacter_Base` (`ActorComponent.GetOwner` _array_element_2)))
      (if (`|EnumInequality` (`SendCharacter.FactionType` _asbp_send_character_base_2) (`self.FactionType`))
        (`KismetArrayLibrary.Array_AddUnique` (`self.EnemiesInRange`) _asbp_send_character_base_2)))))

(fn `UserConstructionScript`
  (`SphereComponent.SetSphereRadius` (`self.AttackIndicator`) (`|GetArrayItem` (`self.AttackRange`)) true))